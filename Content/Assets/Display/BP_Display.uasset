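; Puzzle display that tallies item weight toward a target and removes a barrier when the target is met exactly.
; It adds sizes from BP_KOR's dispatcher only while the player overlaps its box collision.
; Exceeding the target calls GM_Puzzle Retry, while an exact match deactivates the display and destroys BarrierTag actors after a delay.
; A W_Score widget shows color-coded progress on trigger overlap or count changes, resetting on exit or timer.
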(event `self.ReceiveBeginPlay`
  (bind _asbp_kor (cast `/Game/Robo/BP_KOR` (`GameplayStatics.GetPlayerCharacter` 0)))
  (set `self.playerRef` _asbp_kor)
  (add `/Game/Robo/BP_KOR.SendItemSizeDispatcher` _asbp_kor (delegate `UpdateSizeCount`))
  (`self.ResetDisplayText` (struct :`R` 0.6 :`B` 1.0 :`A` 1.0)))

(event `UpdateSizeCount`
  (params (itemSize :type "Float (double-precision)"))
  (if (`PrimitiveComponent.IsOverlappingActor` (`self.BoxCollision`) (`self.playerRef`))
    (set `self.weightCount` (+ (`self.weightCount`) itemSize))
    (`self.CheckScore`)))

(event `self.TextTrigger.OnComponentBeginOverlap`
  (params (OverlappedComponent :type "PrimitiveComponent Object Reference") (OtherActor :type "Actor Object Reference") (OtherComp :type "PrimitiveComponent Object Reference") (OtherBodyIndex :type Integer) (bFromSweep :type Boolean) (SweepResult :type "HitResult Structure (by ref)"))
  (cast `/Game/Robo/BP_KOR` OtherActor)
  (if (`self.bActive`)
    (`self.Update Display Text` (struct :`R` 1.0 :`A` 1.0))))

(event `self.TextTrigger.OnComponentEndOverlap`
  (params (OverlappedComponent :type "PrimitiveComponent Object Reference") (OtherActor :type "Actor Object Reference") (OtherComp :type "PrimitiveComponent Object Reference") (OtherBodyIndex :type Integer))
  (cast `/Game/Robo/BP_KOR` OtherActor)
  (if (`self.bActive`)
    (`self.ResetDisplayText` (struct :`R` 0.6 :`B` 1.0 :`A` 1.0))))

(event `CheckScore`
  (`KismetSystemLibrary.K2_ClearAndInvalidateTimerHandle` (`self.timerHandler`))
  (if (> (`self.weightCount`) (`self.maxWeight`))
    (`self.Update Display Text` (struct :`R` 1.0 :`A` 1.0))
    (bind _asgm_puzzle (cast `/Game/WorldSettings/GM_Puzzle` (`GameplayStatics.GetGameMode`)))
    (`/Game/WorldSettings/GM_Puzzle.Retry` _asgm_puzzle)
    (elif (== (`self.weightCount`) (`self.maxWeight`))
      (`self.Update Display Text` (struct :`G` 1.0 :`A` 1.0))
      (set `self.bActive` false)
      (`KismetSystemLibrary.RetriggerableDelay` 2.0)
      (bind _outactors (`GameplayStatics.GetAllActorsWithTag` (`self.barrierTag`)))
      (`self.K2_DestroyActor` _outactors)
      (`self.FinishDisplayText` (struct :`R` 0.6 :`B` 1.0 :`A` 1.0))
      (else
        (`self.Update Display Text` (struct :`R` 1.0 :`A` 1.0))
        (bind _returnvalue (`KismetSystemLibrary.K2_SetTimerDelegate` (delegate `ResetDisplay`) 2.0))
        (set `self.timerHandler` _returnvalue)))))

(event `ResetDisplay`
  (`self.ResetDisplayText` (struct :`R` 0.6 :`B` 1.0 :`A` 1.0)))

(fn `FinishDisplayText`
  (params (inColor :type "LinearColor Structure"))
  (bind _asw_score (cast `/Game/UI/W_Score` (`WidgetComponent.GetWidget` (`self.Widget`))))
  (bind _displaytext (`/Game/UI/W_Score.displayText` _asw_score))
  (`TextBlock.SetText` _displaytext "Barrier Deactivated")
  (`TextBlock.SetColorAndOpacity` _displaytext (make `SlateColor` inColor)))

(fn `ResetDisplayText`
  (params (inColor :type "LinearColor Structure"))
  (bind _asw_score (cast `/Game/UI/W_Score` (`WidgetComponent.GetWidget` (`self.Widget`))))
  (bind _displaytext (`/Game/UI/W_Score.displayText` _asw_score))
  (`TextBlock.SetText` _displaytext (`self.defaultText`))
  (`TextBlock.SetColorAndOpacity` _displaytext (make `SlateColor` inColor)))

(fn `Update Display Text`
  (params (inColor :type "LinearColor Structure"))
  (bind _asw_score (cast `/Game/UI/W_Score` (`WidgetComponent.GetWidget` (`self.Widget`))))
  (bind _displaytext (`/Game/UI/W_Score.displayText` _asw_score))
  (`TextBlock.SetText` _displaytext (`KismetTextLibrary.Conv_StringToText` (`KismetStringLibrary.Concat_StrStr` (`KismetStringLibrary.Conv_IntToString` (`KismetMathLibrary.Round` (`self.weightCount`))) "/" (`KismetStringLibrary.Conv_IntToString` (`KismetMathLibrary.Round` (`self.maxWeight`))))))
  (`TextBlock.SetColorAndOpacity` _displaytext (make `SlateColor` inColor)))

(fn `UserConstructionScript`)