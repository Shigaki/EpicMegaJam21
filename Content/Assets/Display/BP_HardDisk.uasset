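; BP_HardDisk is a spinning hard disk pickup that completes the puzzle level when the player touches it.
; A looping timer started on BeginPlay repeatedly decrements the actor's yaw to rotate it without using Tick.
; When an actor tagged Player overlaps the static mesh, a DoOnce gate calls LevelCleared on the GM_Puzzle game mode.
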(event `self.ReceiveBeginPlay`
  (`KismetSystemLibrary.K2_SetTimerDelegate` (delegate `Rotate`) 0.02 true))

(event `Rotate`
  (bind (_returnvalue_roll _returnvalue_pitch _returnvalue_yaw) (`KismetMathLibrary.BreakRotator` (`self.K2_GetActorRotation`)))
  (`self.K2_SetActorRotation` (`KismetMathLibrary.MakeRotator` _returnvalue_roll _returnvalue_pitch (- _returnvalue_yaw 1.0))))

(event `self.StaticMeshComponent.OnComponentBeginOverlap`
  (params (OverlappedComponent :type "PrimitiveComponent Object Reference") (OtherActor :type "Actor Object Reference") (OtherComp :type "PrimitiveComponent Object Reference") (OtherBodyIndex :type Integer) (bFromSweep :type Boolean) (SweepResult :type "HitResult Structure (by ref)"))
  (if (`self.ActorHasTag` OtherActor "Player")
    (`/Engine/EditorBlueprintResources/StandardMacros.DoOnce` false
      (:`Completed`
        (bind _asgm_puzzle (cast `/Game/WorldSettings/GM_Puzzle` (`GameplayStatics.GetGameMode`)))
        (`/Game/WorldSettings/GM_Puzzle.LevelCleared` _asgm_puzzle)))))

(fn `UserConstructionScript`)