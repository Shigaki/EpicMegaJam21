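; Virus hazard that patrols along a wire and infects the player's BP_KOR on overlap, presumably with the shrink effect.
; BeginPlay derives both wire endpoints from the wire mesh's right vector and radius, then starts a looping Patrol timer.
; Patrol flip-flops between two timelines that sweep the virus toward each end, lerping from its current location.
; A GM_Puzzle Retry branch is left unconnected.
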(event `self.BP_WiredVirus.OnComponentBeginOverlap`
  (params (OverlappedComponent :type "PrimitiveComponent Object Reference") (OtherActor :type "Actor Object Reference") (OtherComp :type "PrimitiveComponent Object Reference") (OtherBodyIndex :type Integer) (bFromSweep :type Boolean) (SweepResult :type "HitResult Structure (by ref)"))
  (if (`self.ActorHasTag` OtherActor "Player")
    (bind _asbp_kor (cast `/Game/Robo/BP_KOR` OtherActor))
    (`/Game/Robo/BP_KOR.Infected` _asbp_kor "NewEnumerator1")))

(event `self.ReceiveBeginPlay`
  (bind _sm_wire (`self.SM_Wire`))
  (bind _sm_wire_2 (`self.SM_Wire`))
  (set `self.wireStart` (- (`SceneComponent.K2_GetComponentLocation` _sm_wire_2) (* (`SceneComponent.GetRightVector` _sm_wire_2) (`self.wireRadius`))))
  (set `self.wireEnd` (+ (`SceneComponent.K2_GetComponentLocation` _sm_wire) (* (`SceneComponent.GetRightVector` _sm_wire) (`self.wireRadius`))))
  (`KismetSystemLibrary.K2_SetTimer` null "Patrol" 2.0 true))

(event `Patrol`
  (bind _bp_wiredvirus (`self.BP_WiredVirus`))
  (bind _bp_wiredvirus_2 (`self.BP_WiredVirus`))
  (`/Engine/EditorBlueprintResources/StandardMacros.FlipFlop`
    (:`A`
      (bind (_direction _newtrack_0) (`Timeline|Timeline_0` :!via `PlayFromStart`)
        (:`Update`
          (`SceneComponent.K2_SetWorldLocation` _bp_wiredvirus (`KismetMathLibrary.VLerp` (`SceneComponent.K2_GetComponentLocation` _bp_wiredvirus) (`self.wireEnd`) _newtrack_0) true false))))
    (:`B`
      (bind (_direction_2 _newtrack_0_2) (`Timeline|Timeline_1` :!via `PlayFromStart`)
        (:`Update`
          (`SceneComponent.K2_SetWorldLocation` _bp_wiredvirus_2 (`KismetMathLibrary.VLerp` (`SceneComponent.K2_GetComponentLocation` _bp_wiredvirus_2) (`self.wireStart`) _newtrack_0_2) true false))))))

(fn `UserConstructionScript`)