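; Scannable world actor that shows a progress bar while something scans it.
; On BeginPlay it traces down the mesh's local axis against one object type and moves to the hit location without checking for a hit.
; If the player character owns it, the mesh switches to a custom collision channel.
; Start, update and stop events drive the W_ScanningBar widget, with progress computed as remaining data over item size.
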(event `self.ReceiveBeginPlay`
  (bind _staticmeshcomponent (`self.StaticMeshComponent`))
  (bind _returnvalue (`SceneComponent.K2_GetComponentLocation` _staticmeshcomponent))
  (bind _outhit (`KismetSystemLibrary.LineTraceSingleForObjects` :`Start` _returnvalue :`End` (+ _returnvalue (* (`SceneComponent.GetUpVector` _staticmeshcomponent) -500.0)) :`ObjectTypes` (`|MakeArray` "ObjectTypeQuery9" :!type "EObjectTypeQuery Enum") :`DrawDebugType` "ForDuration"))
  (`self.K2_SetActorLocation` (`.Location` (`GameplayStatics.BreakHitResult` _outhit)))
  (if (== (`self.GetOwner`) (`GameplayStatics.GetPlayerCharacter` 0))
    (`PrimitiveComponent.SetCollisionObjectType` (`self.StaticMeshComponent`) "ECC_GameTraceChannel2")))

(event `/Game/Assets/Scannables/BPI_Scannable.StartScanning`
  (bind _asw_scanning_bar (cast `/Game/UI/W_ScanningBar` (`WidgetComponent.GetUserWidgetObject` (`self.ProgressBar`))))
  (`/Game/UI/W_ScanningBar.ResetProgressBar` _asw_scanning_bar)
  (`SceneComponent.SetVisibility` (`self.ProgressBar`) true false))

(event `/Game/Assets/Scannables/BPI_Scannable.UpdateScanPercent`
  (params (remainingData :type "Float (single-precision)"))
  (bind _asw_scanning_bar (cast `/Game/UI/W_ScanningBar` (`WidgetComponent.GetUserWidgetObject` (`self.ProgressBar`))))
  (`/Game/UI/W_ScanningBar.UpdateProgressBar` _asw_scanning_bar (/ remainingData (`self.itemSize`))))

(event `/Game/Assets/Scannables/BPI_Scannable.StopScanning`
  (`SceneComponent.SetVisibility` (`self.ProgressBar`) false false))

(fn `UserConstructionScript`)