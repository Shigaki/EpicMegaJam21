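; BP_Scannable is a scannable object with a static mesh and a widget that displays scan progress.
; StartScanning resets and shows the W_ScanningBar, UpdateScanPercent fills it from remaining data divided by ItemSize, and StopScanning hides it.
; On BeginPlay, the mesh switches to a custom collision object type if the object's owner is the first player's character.
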(event `self.ReceiveBeginPlay`
  (if (== (`self.GetOwner`) (`GameplayStatics.GetPlayerCharacter` 0))
    (`PrimitiveComponent.SetCollisionObjectType` (`self.StaticMeshComponent`) "ECC_GameTraceChannel2")))

(event `/Game/Assets/BPI_Scannable.StartScanning`
  (bind _asw_scanning_bar (cast `/Game/UI/W_ScanningBar` (`WidgetComponent.GetUserWidgetObject` (`self.Widget`))))
  (`/Game/UI/W_ScanningBar.ResetProgressBar` _asw_scanning_bar)
  (`SceneComponent.SetVisibility` (`self.Widget`) true false))

(event `/Game/Assets/BPI_Scannable.UpdateScanPercent`
  (params (remainingData :type "Float (single-precision)"))
  (bind _asw_scanning_bar (cast `/Game/UI/W_ScanningBar` (`WidgetComponent.GetUserWidgetObject` (`self.Widget`))))
  (`/Game/UI/W_ScanningBar.UpdateProgressBar` _asw_scanning_bar (/ remainingData (`self.itemSize`))))

(event `/Game/Assets/BPI_Scannable.StopScanning`
  (`SceneComponent.SetVisibility` (`self.Widget`) false false))

(fn `UserConstructionScript`)