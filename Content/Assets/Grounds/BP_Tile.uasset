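; BP_Tile is a ground tile that tracks whether it is buildable and shows that state through its mesh material.
; Any begin overlap immediately switches it to M_virus and clears Buildable.
; End overlap, and a half-second delayed check after BeginPlay, run UpdateTileColor, which counts overlapping actors other than SM_Wall and restores the basic tile material and Buildable only when none remain.
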(event `self.ReceiveBeginPlay`
  (`KismetSystemLibrary.Delay` 0.5)
  (`self.UpdateTileColor` (`self.StaticMesh`)))

(event `self.StaticMesh.OnComponentBeginOverlap`
  (params (OverlappedComponent :type "PrimitiveComponent Object Reference") (OtherActor :type "Actor Object Reference") (OtherComp :type "PrimitiveComponent Object Reference") (OtherBodyIndex :type Integer) (bFromSweep :type Boolean) (SweepResult :type "HitResult Structure (by ref)"))
  (`PrimitiveComponent.SetMaterial` OverlappedComponent 0 "/Game/Assets/BasicProps/m_virus.m_virus")
  (set `self.bBuildable` false))

(event `self.StaticMesh.OnComponentEndOverlap`
  (params (OverlappedComponent :type "PrimitiveComponent Object Reference") (OtherActor :type "Actor Object Reference") (OtherComp :type "PrimitiveComponent Object Reference") (OtherBodyIndex :type Integer))
  (`self.UpdateTileColor` OverlappedComponent))

(fn `UpdateTileColor`
  (params (mesh :type "PrimitiveComponent Object Reference"))
  (set `self.countOverlap` 0)
  (for _array_element (`PrimitiveComponent.GetOverlappingActors` mesh null)
    (if (!= _array_element "/Game/Assets/BasicProps/SM_Wall.SM_Wall")
      (`/Engine/EditorBlueprintResources/StandardMacros.IncrementInt` (`self.countOverlap`))))
  (if (> (`self.countOverlap`) 0)
    (`PrimitiveComponent.SetMaterial` mesh 0 "/Game/Assets/BasicProps/m_virus.m_virus")
    (set `self.bBuildable` false)
    (else
      (`PrimitiveComponent.SetMaterial` mesh 0 "/Game/Assets/BasicProps/M_BasicEmitter_Tile.M_BasicEmitter_Tile")
      (set `self.bBuildable` true))))

(fn `UserConstructionScript`)