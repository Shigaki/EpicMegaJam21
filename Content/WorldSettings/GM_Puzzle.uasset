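; Puzzle game mode that tracks the level's tile grid and handles level retries.
; On BeginPlay it caches all BP_Tile actors, hides their meshes and stores the BP_KOR player reference; ToggleGridVisibility shows or hides the grid.
; GetClosestTile linearly searches the cached tiles by distance to a position, but never initializes ClosestTile to the first tile.
; Retry prints a message, waits briefly, then reopens the current level.
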(event `self.ReceiveBeginPlay`
  (`self.GetTilesRef`)
  (bind _asbp_kor (cast `/Game/Robo/BP_KOR` (`GameplayStatics.GetPlayerCharacter` 0)))
  (set `self.playerRef` _asbp_kor))

(event `ToggleGridVisibility`
  (params (visible :type Boolean))
  (if visible
    (for _array_element (`self.Tiles`)
      (`SceneComponent.SetVisibility` (`/Game/Assets/Grounds/BP_Tile.StaticMesh` _array_element) true false))
    (else
      (for _array_element_2 (`self.Tiles`)
        (`SceneComponent.SetVisibility` (`/Game/Assets/Grounds/BP_Tile.StaticMesh` _array_element_2) false false)))))

(event `Retry`
  (`KismetSystemLibrary.PrintString` "Initializing Factory Reset")
  (`KismetSystemLibrary.Delay` 2.0)
  (bind _returnvalue (`GameplayStatics.GetCurrentLevelName` true))
  (`GameplayStatics.OpenLevel` (`KismetStringLibrary.Conv_StringToName` _returnvalue)))

(fn `GetClosestTile`
  (params (inPosition :type "Vector Structure"))
  (returns (outTile :type "/Game/Assets/Grounds/BP_Tile Object Reference"))
  (locals (closestPosition :type "Vector Structure") (closestDistance :type "Float (double-precision)" :default 0.0) (closestTile :type "/Game/Assets/Grounds/BP_Tile Object Reference"))
  (bind _returnvalue (`self.K2_GetActorLocation` (`|GetArrayItem` (`self.Tiles`))))
  (set `local.closestPosition` _returnvalue)
  (set `local.closestDistance` (`KismetMathLibrary.Vector_Distance` inPosition _returnvalue))
  (for _array_element (`self.Tiles`)
    (bind _returnvalue_2 (`self.K2_GetActorLocation` _array_element))
    (bind _returnvalue_3 (`KismetMathLibrary.Vector_Distance` _returnvalue_2 inPosition))
    (if (< _returnvalue_3 (`local.closestDistance`))
      (set `local.closestPosition` _returnvalue_2)
      (set `local.closestDistance` _returnvalue_3)
      (set `local.closestTile` _array_element)))
  (return (`local.closestTile`)))

(fn `GetTilesRef`
  (bind _outactors (`GameplayStatics.GetAllActorsOfClass` "/Game/Assets/Grounds/BP_Tile.BP_Tile_C"))
  (bind _output_get (set `self.Tiles` _outactors))
  (for _array_element _output_get
    (`SceneComponent.SetVisibility` (`/Game/Assets/Grounds/BP_Tile.StaticMesh` _array_element) false false)))

(fn `UserConstructionScript`)