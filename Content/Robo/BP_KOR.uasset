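; Player robot character that scans items in the world and clones them, with diagonal-mapped movement and jumping.
; Holding scan line-traces ahead for a BP_Scannable, then a looping timer drains its size by ReadSpeed; moving, jumping or releasing cancels.
; Completed scans change collision channel and join ScannedItems, from which Clone spawns a random item's class ahead and dispatches its size.
; UI events forward disk size and used space to PlayerHUD.
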(event `self.ReceiveBeginPlay`
  (`ActorComponent.Activate` (`self.Camera1`) false))

(event `UI_UpdateDiskUsedSpace`
  (params (diskUsedSpace :type "Float (double-precision)"))
  ;[1 1 1] Update UI Info
  (bind _asplayer_controller (cast `PlayerController` (`self.GetController`)))
  (bind _asplayer_hud (cast `/Game/UI/PlayerHUD` (`PlayerController.GetHUD` _asplayer_controller)))
  (`TextBlock.SetText` (`/Game/UI/W_PlayerInterface.UsedSpace` (`/Game/UI/PlayerHUD.playerUI` _asplayer_hud)) (`KismetTextLibrary.Conv_DoubleToText` diskUsedSpace "HalfToEven")))

(event `InputAxis|MoveForward`
  (params (AxisValue :type "Float (single-precision)"))
  ;[1 0.368 1] Input
  (if (!= AxisValue 0.0)
    (`self.CancelScanAction`)
    (`self.AddMovementInput` (+ (`KismetMathLibrary.Vector_Forward`) (`KismetMathLibrary.Vector_Left`)) AxisValue)))

(event `InputAxis|MoveRight`
  (params (AxisValue :type "Float (single-precision)"))
  ;[1 0.368 1] Input
  (if (!= AxisValue 0.0)
    (`self.CancelScanAction`)
    (`self.AddMovementInput` (+ (`KismetMathLibrary.Vector_Right`) (`KismetMathLibrary.Vector_Forward`)) AxisValue)))

(event `UI_SetDiskSize`
  (params (diskSize :type "Float (double-precision)"))
  ;[1 1 1] Update UI Info
  (bind _asplayer_controller (cast `PlayerController` (`self.GetController`)))
  (bind _asplayer_hud (cast `/Game/UI/PlayerHUD` (`PlayerController.GetHUD` _asplayer_controller)))
  (`/Game/UI/PlayerHUD.InitPlayerUI` _asplayer_hud diskSize))

(event `InputAction|Jump`
  (params (Key :type "Key Structure"))
  ;[1 0.368 1] Input
  (:`Pressed`
    (`self.CancelScanAction`)
    (`self.Jump`))
  (:`Released`
    (`self.StopJumping`)))

(event `InputAction|ScanItem`
  (params (Key :type "Key Structure"))
  (bind _scanningitem (`self.scanningItem`))
  ;[-0.08 1 0.192] Scan
  (:`Pressed`
    (bind (_startpoint _endpoint) (`self.GetInteractLineTrace` (`self.interactDistance`)))
    (bind (_outhit _returnvalue) (`KismetSystemLibrary.LineTraceSingleForObjects` :`Start` _startpoint :`End` _endpoint :`ObjectTypes` (`self.Object Types`) :`DrawDebugType` "ForDuration"))
    (if _returnvalue
      (bind _asbp_scannable (cast `/Game/Assets/BP_Scannable` (`.HitActor` (`GameplayStatics.BreakHitResult` _outhit))))
      (set `self.scanningItem` _asbp_scannable)
      (set `self.bScanning` true)
      (set `self.scanRemainingData` (`/Game/Assets/BP_Scannable.itemSize` _scanningitem))
      (`/Game/Assets/BP_Scannable.StartScanning` _scanningitem)
      (bind _returnvalue_2 (`KismetSystemLibrary.K2_SetTimer` null "ScanningData" 0.02 true))
      (set `self.scanHandler` _returnvalue_2)))
  (:`Released`
    (`self.CancelScanAction`)))

(event `ScanningData`
  ;[-0.08 1 0.192] Scan
  (bind _output_get (set `self.scanRemainingData` (- (`self.scanRemainingData`) (* (`self.readSpeed`) 0.02))))
  (`/Game/Assets/BP_Scannable.UpdateScanPercent` (`self.scanningItem`) _output_get)
  (if (<= _output_get 0.0)
    (`self.CancelScanAction`)
    (`PrimitiveComponent.SetCollisionObjectType` (`StaticMeshActor.StaticMeshComponent` (`self.scanningItem`)) "ECC_GameTraceChannel2")
    (`BlueprintSetLibrary.Set_AddItems` (`self.ScannedItems`) (`|MakeArray` (`self.scanningItem`)))))

(event `InputAction|CloneItem`
  (params (Key :type "Key Structure"))
  ;[-0.44 1 1] Clone
  (:`Pressed`
    (bind _result (`BlueprintSetLibrary.Set_ToArray` (`self.ScannedItems`)))
    (bind _output (`|GetArrayItem` _result (`KismetMathLibrary.RandomIntegerInRange` 0 (- (`KismetArrayLibrary.Array_Length` _result) 1))))
    (`/Engine/EditorBlueprintResources/StandardMacros.IsValid` _output
      (:`Is Valid`
        (bind _output_get (set `self.spawnedItem` _output))
        (bind (_startpoint _endpoint) (`self.GetInteractLineTrace` (`self.interactDistance`)))
        (`|SpawnActorFromClass` (`GameplayStatics.GetObjectClass` _output_get) (`KismetMathLibrary.MakeTransform` _endpoint) "AdjustIfPossibleButAlwaysSpawn" "OverrideRootScale" self null)
        (`self.SendItemSizeDispatcher` (`/Game/Assets/BP_Scannable.itemSize` (`self.spawnedItem`)))))))

(fn `CancelScanAction`
  (bind _scanhandler (`self.scanHandler`))
  (if (`KismetSystemLibrary.K2_IsValidTimerHandle` _scanhandler)
    (`KismetSystemLibrary.K2_ClearAndInvalidateTimerHandle` _scanhandler)
    (`/Game/Assets/BP_Scannable.StopScanning` (`self.scanningItem`))
    (set `self.bScanning` false)))

(fn `GetInteractLineTrace`
  (params (distance :type "Float (double-precision)"))
  (returns (startPoint :type "Vector Structure") (endPoint :type "Vector Structure"))
  (locals (lineDistance :type "Float (double-precision)"))
  (bind _capsulecomponent (`self.CapsuleComponent`))
  (bind (_returnvalue_x _returnvalue_y) (`KismetMathLibrary.BreakVector` (`SceneComponent.GetForwardVector` _capsulecomponent)))
  (bind _returnvalue (+ (`SceneComponent.K2_GetComponentLocation` _capsulecomponent) (0.0 0.0 -25.0)))
  (set `local.lineDistance` distance)
  (return _returnvalue (+ _returnvalue (`KismetMathLibrary.MakeVector` (* _returnvalue_x (`local.lineDistance`)) (* _returnvalue_y (`local.lineDistance`))))))

(fn `UserConstructionScript`)